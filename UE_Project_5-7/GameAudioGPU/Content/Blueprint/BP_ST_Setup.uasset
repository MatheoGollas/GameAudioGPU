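; Test setup actor for GPU sound tracing that populates the level with BP_ST_Emitter actors and reports the concurrent ray count.
; BeginPlay spawns emitters at random points in a box around the actor, with a fixed or random ray type (Direct, Shower, Hedgehog).
; It then configures and starts tracing through AudioGPUSubsystem.
; UpdateSoundTracingParams reapplies the parameters and reprints the total, counting Direct emitters as one ray each.
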(event Custom|UpdateSoundTracingParams
  (bind _returnvalue (Game|GetPlayerController 0))
  (bind _returnvalue_2 (Subsystems|GetAudioGPUSubsystem _returnvalue))
  (Utilities|IsValid _returnvalue
    (:Is%20Valid
      (Utilities|IsValid _returnvalue_2
        (:Is%20Valid
          (Class|AudioGPUSubsystem|SetSoundTracingParams _returnvalue_2 (Variables|SoundTracingParams|GetNum%20Rays%20Per%20Emitter) (Variables|SoundTracingParams|GetShower%20Radius) (Variables|SoundTracingParams|GetDefault%20Ray%20Length) (Variables|SoundTracingParams|GetFrame%20Skips))
          (Development|PrintString (Utilities|String|Append "Concurrent rays: " (Utilities|String|ToString(Integer) (+ (* (Variables|Default|GetPatternEmitterAmount) (Variables|SoundTracingParams|GetNum%20Rays%20Per%20Emitter)) (Variables|Default|GetSingleEmitterAmount)))) true true "(R=0.000000,G=1.000000,B=0.406584,A=1.000000)"))))))

(event EventBeginPlay
  (bind _returnvalue (Game|GetPlayerController 0))
  (bind _returnvalue_2 (Subsystems|GetAudioGPUSubsystem _returnvalue))
  (for _index (range 0 (- (Math|Integer|Max(Integer) (Variables|Default|GetEmitterAmount)) 1))
    (bind _output_get (Variables|Default|SetTempVar (select (Variables|Default|GetRandomEmitterType) (Utilities|Select :Index (Math|Random|RandomIntegerinRange 0 2) :Option%200 "Direct" :Option%201 "Shower" :Option%202 "Hedgehog") (Variables|Default|GetEmitterType))))
    (Game|SpawnActorfromClass "/Game/Blueprint/BP_ST_Emitter.BP_ST_Emitter_C" (Math|Transform|MakeTransform (Math|Random|RandomPointinBoundingBox (+ (Transformation|GetWorldLocation (Variables|Default|GetDefaultSceneRoot)) "0.000000,0.000000,100.000000") "4500.000000,4500.000000,100.000000") "0, 0, 0" "1.000000,1.000000,1.000000") "AlwaysSpawn" "MultiplyWithRoot" 0 _output_get (Variables|Default|GetDebug) 0)
    (if (Utilities|Enum|Equal(Enum) (Variables|Default|GetTempVar) "Direct")
      (Math|Integer|IncrementInt (Variables|Default|GetSingleEmitterAmount))
      (else
        (Math|Integer|IncrementInt (Variables|Default|GetPatternEmitterAmount)))))
  (Class|AudioGPUSubsystem|SetSoundTracingParams _returnvalue_2 (Variables|SoundTracingParams|GetNum%20Rays%20Per%20Emitter) (Variables|SoundTracingParams|GetShower%20Radius) (Variables|SoundTracingParams|GetDefault%20Ray%20Length) (Variables|SoundTracingParams|GetFrame%20Skips))
  (Class|AudioGPUSubsystem|StartSoundTracing _returnvalue_2)
  (Development|PrintString (Utilities|String|Append "Concurrent rays: " (Utilities|String|ToString(Integer) (+ (* (Variables|Default|GetPatternEmitterAmount) (Variables|SoundTracingParams|GetNum%20Rays%20Per%20Emitter)) (Variables|Default|GetSingleEmitterAmount)))) true true "(R=0.000000,G=1.000000,B=0.406584,A=1.000000)"))

(event EventTick
  (params (DeltaSeconds :type Float%20%28single-precision%29)))

(fn ConstructionScript)