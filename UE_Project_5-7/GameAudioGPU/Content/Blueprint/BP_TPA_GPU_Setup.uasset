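; BP_TPA_GPU_Setup is an actor that sets up GPU third-person audio (TPA) emitters for what appears to be an audio test.
; On BeginPlay it spawns EmitterAmount BP_ThirdPersonEmitterGPU actors at its own root transform, passing each the UseCPU flag.
; Each tick it calls UpdateTPAEmitters on the player controller's AudioGPUSubsystem, with ticking disabled when UseCPU is set.
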(event EventBeginPlay
  (if (Variables|Default|GetUseCPU)
    (Actor|Tick|SetActorTickEnabled false))
  (for _index (range 0 (Math|Integer|Max(Integer) (Variables|Default|GetEmitterAmount)))
    (Game|SpawnActorfromClass "/Game/Blueprint/BP_ThirdPersonEmitterGPU.BP_ThirdPersonEmitterGPU_C" (Transformation|GetWorldTransform (Variables|Default|GetDefaultSceneRoot)) "AlwaysSpawn" "MultiplyWithRoot" 0 (Variables|Default|GetUseCPU) 0)))

(event Collision|EventActorBeginOverlap
  (params (OtherActor :type Actor%20Object%20Reference)))

(event EventTick
  (params (DeltaSeconds :type Float%20%28single-precision%29))
  (Class|AudioGPUSubsystem|UpdateTPAEmitters (Subsystems|GetAudioGPUSubsystem (Game|GetPlayerController 0))))

(fn ConstructionScript)