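; BP_ST_Emitter is an audio emitter actor that registers with the AudioGPUSubsystem for sound tracing and visualizes the results.
; On BeginPlay it adds itself to the subsystem's emitter buffer, exposing its root component through GetComponent.
; SoundTraceData unpacks a packed vector into hit position (XYZ) and hit flag (W).
; Tick draws a debug sphere at the emitter and a line to that position, colored by hit state.
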(event EventBeginPlay
  (bind _returnvalue (Game|GetPlayerController 0))
  (bind _returnvalue_2 (Subsystems|GetAudioGPUSubsystem _returnvalue))
  (bind _asaudio_emitter_gpu (Utilities|Casting|CastToAudioEmitterGPU self)
    (:then
      (Class|AudioGPUSubsystem|AddEmittertoBuffer _returnvalue_2 _asaudio_emitter_gpu))
    (:CastFailed
      (Class|AudioGPUSubsystem|AddEmittertoBuffer _returnvalue_2 self))))

(event Collision|EventActorBeginOverlap
  (params (OtherActor :type Actor%20Object%20Reference)))

(event EventTick
  (params (DeltaSeconds :type Float%20%28single-precision%29))
  (bind _defaultsceneroot (Variables|Default|GetDefaultSceneRoot))
  (bind _returnvalue (Transformation|GetWorldLocation _defaultsceneroot))
  (Rendering|Debug|DrawDebugSphere _returnvalue 1e+01 12 "(R=1.000000,G=0.000000,B=0.061136,A=1.000000)" 0.0)
  (Rendering|Debug|DrawDebugLine _returnvalue (Variables|Default|GetRayHit) (Math|Color|SelectColor "(R=1.000000,G=0.155021,B=0.119200,A=1.000000)" "(R=0.341711,G=1.000000,B=0.291993,A=1.000000)" (Variables|Default|GetIsHitting)) 0.0 0.0))

(event EventSoundTraceData
  (params (Data :type Sound%20Trace%20Result%20Structure%20%28by%20ref%29))
  (Variables|Default|SetRayHit (Math|Vector|MakeVector (.x (.wpos_didhit Data)) (.y (.wpos_didhit Data)) (.z (.wpos_didhit Data))))
  (Variables|Default|SetIsHitting (> (.w (.wpos_didhit Data)) 0.1)))

(fn ConstructionScript)

(fn GetComponent
  (return (Variables|Default|GetDefaultSceneRoot)))